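; TPSPlayerController is a player controller for a third-person game that supplies a view location and an aim direction.
; Viewpoint returns the FollowCamera location of the controlled ThirdPersonCharacter, falling back to the controller's focal location for any other pawn.
; AimVector returns the forward vector of the controlled pawn's base aim rotation.
; The event graph and construction script contain no active logic.
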(fn `AimVector`
  (returns (NewParam :type "Vector Structure"))
  (locals (outAim :type "Vector Structure"))
  (set `local.outAim` (`KismetMathLibrary.GetForwardVector` (`Pawn.GetBaseAimRotation` (`self.K2_GetPawn`))))
  (return (`local.outAim`)))

(fn `UserConstructionScript`)

(fn `Viewpoint`
  (returns (NewParam :type "Vector Structure"))
  (set `self.OutViewLocation` (0.0 0.0 0.0))
  (bind _asthird_person_character (cast `/Game/ThirdPersonBP/Blueprints/ThirdPersonCharacter` (`self.K2_GetPawn`))
    (:`then`
      (bind _desiredview (`CameraComponent.GetCameraView` (`/Game/ThirdPersonBP/Blueprints/ThirdPersonCharacter.FollowCamera` _asthird_person_character) 0.0))
      (set `self.OutViewLocation` (break `MinimalViewInfo` _desiredview)))
    (:`CastFailed`
      (set `self.OutViewLocation` (`self.GetFocalLocation`))))
  (return (`self.OutViewLocation`)))